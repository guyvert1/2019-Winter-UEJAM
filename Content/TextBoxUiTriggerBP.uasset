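; One-shot trigger actor that shows a text message on the player's screen when an actor overlaps it.
; On first overlap it sets a Triggered flag, then casts player 0's pawn to TestCharacter without checking which actor overlapped.
; It fills the character's TextUI widget with its Text, displays it and disables the character's input.
; After a five-second delay it removes the widget and re-enables input.
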(event EventBeginPlay)

(event Collision|EventActorBeginOverlap
  (params (OtherActor :type Actor%20Object%20Reference))
  (bind _returnvalue (Game|GetPlayerController 0))
  (if (not (Variables|Default|GetTriggered))
    (Variables|Default|SetTriggered true)
    (bind _astest_character (Utilities|Casting|CastToTestCharacter (Pawn|GetControlledPawn _returnvalue)))
    (Default|SetText (Variables|/Game/ThirdPersonBP/Blueprints/TestCharacter.TestCharacter_C|GetTextUI _astest_character) (Variables|Default|GetText))
    (UserInterface|Viewport|AddtoViewport (Variables|/Game/ThirdPersonBP/Blueprints/TestCharacter.TestCharacter_C|GetTextUI _astest_character) 0)
    (Input|DisableInput _astest_character _returnvalue)
    (Utilities|FlowControl|Delay 5.0)
    (Widget|RemovefromParent (Variables|/Game/ThirdPersonBP/Blueprints/TestCharacter.TestCharacter_C|GetTextUI _astest_character))
    (Input|EnableInput _returnvalue _returnvalue)))

(event EventTick
  (params (DeltaSeconds :type Float%20%28single-precision%29)))

(fn ConstructionScript)