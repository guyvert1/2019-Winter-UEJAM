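; AreaOneDoor is a barrier for the first area that appears when enemies spawn and is removed once they are defeated.
; Its mesh is hidden on BeginPlay, and EnemiesSpawned shows it with query and physics collision.
; EnemyiesDefeated finds the first FinalDoor actor, removes the last entry from its Doors array, then destroys this door.
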(event EventBeginPlay
  (Rendering|SetVisibility (Variables|Debug|GetStaticMeshComponent) false false))

(event Collision|EventActorBeginOverlap
  (params (OtherActor :type Actor%20Object%20Reference)))

(event EventTick
  (params (DeltaSeconds :type Float%20%28single-precision%29)))

(fn ConstructionScript)

(fn EnemyiesDefeated
  (bind _outactors (Actor|GetAllActorsOfClass "/Game/FinalDoor.FinalDoor_C"))
  (Utilities|Array|RemoveIndex (Variables|/Game/FinalDoor.FinalDoor_C|GetDoors (Utilities|Array|Get(acopy) _outactors)) (- (Utilities|Array|Length (Variables|/Game/FinalDoor.FinalDoor_C|GetDoors (Utilities|Array|Get(acopy) _outactors))) 1))
  (Actor|DestroyActor))

(fn EnemiesSpawned
  (bind _staticmeshcomponent (Variables|Debug|GetStaticMeshComponent))
  (Rendering|SetVisibility _staticmeshcomponent true false)
  (Collision|SetCollisionEnabled _staticmeshcomponent "QueryAndPhysics"))